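; Base projectile Blueprint that handles the cosmetic sound and visual effects for a projectile's launch, flight and impact.
; BeginPlay plays the spawn sound, attaches the flight sound to the root and spawns a muzzle effect facing the actor's forward vector.
; OnSpawnProjectileHitFX plays the impact sound and effect at the given hit location.
; Each asset is optional, and Niagara systems take priority over Cascade particle fallbacks.
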(event `self.ReceiveBeginPlay`
  (bind _returnvalue (`self.K2_GetActorLocation`))
  (bind _returnvalue_2 (`KismetMathLibrary.Conv_VectorToRotator` (`self.GetActorForwardVector`)))
  (`|ExecutionSequence`
    (:`then_0`
      (bind _projectilespawnsound (`self.ProjectileSpawnSound`)
        (:`then`
          (`GameplayStatics.PlaySoundAtLocation` _projectilespawnsound (`self.K2_GetActorLocation`) (struct) 1.0 1.0 0.0 null null null null))
        (:`else`)))
    (:`then_1`
      (bind _projectileflysound (`self.ProjectileFlySound`)
        (:`then`
          (`GameplayStatics.SpawnSoundAttached` _projectileflysound (`self.RootComponent`) "None" (0.0 0.0 0.0) (struct) "KeepRelativeOffset" true 1.0 1.0 0.0 null null))
        (:`else`)))
    (:`then_2`
      (bind _projectilemuzzlenaigarafx (`self.ProjectileMuzzleNaigaraFX`)
        (:`then`
          (`NiagaraFunctionLibrary.SpawnSystemAtLocation` _projectilemuzzlenaigarafx _returnvalue _returnvalue_2))
        (:`else`
          (bind _projectilemuzzleparticlefx (`self.ProjectileMuzzleParticleFX`)
            (:`then`
              (`GameplayStatics.SpawnEmitterAtLocation` _projectilemuzzleparticlefx _returnvalue _returnvalue_2))
            (:`else`)))))))

(event `self.BP_OnSpawnProjectileHitFX`
  (params (HitLocation :type "Vector Structure (by ref)"))
  (`|ExecutionSequence`
    (:`then_0`
      (bind _projectileimpactsound (`self.ProjectileImpactSound`)
        (:`then`
          (`GameplayStatics.PlaySoundAtLocation` _projectileimpactsound HitLocation (struct) 1.0 1.0 0.0 null null null null))
        (:`else`)))
    (:`then_1`
      (bind _projectileimpactnaigarafx (`self.ProjectileImpactNaigaraFX`)
        (:`then`
          (`NiagaraFunctionLibrary.SpawnSystemAtLocation` _projectileimpactnaigarafx HitLocation))
        (:`else`
          (bind _projectileimpactparticlefx (`self.ProjectileImpactParticleFX`)
            (:`then`
              (`GameplayStatics.SpawnEmitterAtLocation` _projectileimpactparticlefx HitLocation))
            (:`else`)))))))

(fn `UserConstructionScript`)